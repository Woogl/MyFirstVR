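; VR hand actor that follows a motion controller and grabs objects, with a LeftHand flag that mirrors the mesh and switches the motion source.
; OnGrab runs a zero-length, debug-drawn sphere trace at the controller to find a BP_GrabComponent, then stores it if TryGrab succeeds.
; OnRelease calls TryRelease on the held component without clearing the reference.
; Both set ABP_Hand's grasp alpha, even when nothing is held.
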(event `self.ReceiveBeginPlay`
  (if (`self.LeftHand`)
    (`SceneComponent.SetRelativeScale3D` (`self.HandMesh`) (1.0 1.0 -1.0))
    (set `MotionControllerComponent.MotionSource` "Left" (`self.MotionController`))))

(fn `FindGrabComponentNearHand`
  (returns (GrabComponent :type "/Game/Blueprints/BP_GrabComponent Object Reference"))
  (locals (LocalGrabLocation :type "Vector Structure" :default (0.0 0.0 0.0)) (LocalGrabComponent :type "/Game/Blueprints/BP_GrabComponent Object Reference"))
  (`|ExecutionSequence`
    (:`then_0`
      (bind _output_get (set `local.LocalGrabLocation` (`SceneComponent.K2_GetComponentLocation` (`self.MotionController`))))
      (bind (_outhit _returnvalue) (`KismetSystemLibrary.SphereTraceSingleForObjects` :`Start` _output_get :`End` _output_get :`Radius` (`self.GrabRadius`) :`ObjectTypes` (`|MakeArray` "ObjectTypeQuery7" :!type "EObjectTypeQuery Enum") :`DrawDebugType` "ForDuration"))
      (if _returnvalue
        (bind _returnvalue_2 (`self.GetComponentByClass` (`.HitActor` (`GameplayStatics.BreakHitResult` _outhit)) "/Game/Blueprints/BP_GrabComponent.BP_GrabComponent_C"))
        (`/Engine/EditorBlueprintResources/StandardMacros.IsValid` _returnvalue_2
          (:`Is Valid`
            (set `local.LocalGrabComponent` _returnvalue_2)))))
    (:`then_1`
      (return (`local.LocalGrabComponent`)))))

(fn `OnGrab`
  (`|ExecutionSequence`
    (:`then_0`
      (bind _grabcomponent (`self.FindGrabComponentNearHand`))
      (`/Engine/EditorBlueprintResources/StandardMacros.IsValid` _grabcomponent
        (:`Is Valid`
          (bind _success (`/Game/Blueprints/BP_GrabComponent.TryGrab` _grabcomponent self))
          (if _success
            (set `self.HeldComponent` _grabcomponent)))))
    (:`then_1`
      (bind _asabp_hand (cast `/Game/Resources/Hand/ABP_Hand` (`SkeletalMeshComponent.GetAnimInstance` (`self.HandMesh`))))
      (set `/Game/Resources/Hand/ABP_Hand.PoseAlphaGrasp` 1.0 _asabp_hand))))

(fn `OnRelease`
  (bind _heldcomponent (`self.HeldComponent`))
  (`|ExecutionSequence`
    (:`then_0`
      (`/Engine/EditorBlueprintResources/StandardMacros.IsValid` _heldcomponent
        (:`Is Valid`
          (`/Game/Blueprints/BP_GrabComponent.TryRelease` _heldcomponent))))
    (:`then_1`
      (bind _asabp_hand (cast `/Game/Resources/Hand/ABP_Hand` (`SkeletalMeshComponent.GetAnimInstance` (`self.HandMesh`))))
      (set `/Game/Resources/Hand/ABP_Hand.PoseAlphaGrasp` 0.0 _asabp_hand))))

(fn `UserConstructionScript`)